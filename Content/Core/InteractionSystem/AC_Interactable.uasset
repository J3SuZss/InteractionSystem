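; AC_Interactable is an interaction component that highlights a mesh while it is hovered.
; CE_OnHover casts the passed primitive to StaticMeshComponent, falling back to MeshComponent, and applies OverlayMaterial as its overlay material.
; CE_OnUnHover runs the same casts and clears the overlay.
; The component only handles this visual feedback, with no interaction logic in its event graph.
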(event Custom|CE_OnHover
  (params (NewParam :type Actor%20Object%20Reference) (PrimRef :type Primitive%20Component%20Object%20Reference))
  (bind _asstatic_mesh_component (Utilities|Casting|CastToStaticMeshComponent PrimRef)
    (:then
      (Rendering|Material|SetOverlayMaterial _asstatic_mesh_component (Variables|Default|GetOverlayMaterial) :!class /Script/Engine.MeshComponent))
    (:CastFailed
      (bind _asmesh_component (Utilities|Casting|CastToMeshComponent PrimRef))
      (Rendering|Material|SetOverlayMaterial _asmesh_component (Variables|Default|GetOverlayMaterial) :!class /Script/Engine.MeshComponent))))

(event Custom|CE_OnUnHover
  (params (PrimRef :type Primitive%20Component%20Object%20Reference))
  (bind _asstatic_mesh_component (Utilities|Casting|CastToStaticMeshComponent PrimRef)
    (:then
      (Rendering|Material|SetOverlayMaterial _asstatic_mesh_component 0 :!class /Script/Engine.MeshComponent))
    (:CastFailed
      (bind _asmesh_component (Utilities|Casting|CastToMeshComponent PrimRef))
      (Rendering|Material|SetOverlayMaterial _asmesh_component 0 :!class /Script/Engine.MeshComponent))))