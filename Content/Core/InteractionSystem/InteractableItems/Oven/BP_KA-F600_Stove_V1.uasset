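; BP_KA-F600_Stove_V1 is an interactable stove with an opening door and a toggleable burner effect.
; OnInteraction branches on the tag of the component passed in, with a FlipFlop alternating each action.
; "Door" plays or reverses a Timeline that lerps the door mesh's relative roll between closed and open.
; "Ocak" (Turkish for stove) shows or hides the Niagara component.
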(event EventBeginPlay)

(event Collision|EventActorBeginOverlap
  (params (OtherActor :type Actor%20Object%20Reference)))

(event EventTick
  (params (DeltaSeconds :type Float%20%28single-precision%29)))

(event EventOnInteraction
  (params (PrimRef :type Primitive%20Component%20Object%20Reference))
  (bind _sm_ka_f600_stove_v1_door (Variables|Default|GetSM_KA-F600_Stove_V1_Door))
  (bind _returnvalue (Transformation|GetRelativeTransform _sm_ka_f600_stove_v1_door))
  (if (Components|ComponentHasTag PrimRef "Door")
    (Utilities|FlowControl|FlipFlop
      (:A
        (bind _newtrack_0 (Timeline|Timeline Play)
          (:Update
            (Transformation|SetRelativeRotation _sm_ka_f600_stove_v1_door (Math|Rotator|MakeRotator (Math|Float|Lerp 0.0 9e+01 _newtrack_0) (.pitch (.rotation _returnvalue)) (.yaw (.rotation _returnvalue))) false false))))
      (:B
        (Timeline|Timeline Reverse)))
    (elif (Components|ComponentHasTag PrimRef "Ocak")
      (Utilities|FlowControl|FlipFlop
        (:A
          (Rendering|SetVisibility (Variables|Default|GetNiagara) true false))
        (:B
          (Rendering|SetVisibility (Variables|Default|GetNiagara) false false))))))

(fn ConstructionScript)