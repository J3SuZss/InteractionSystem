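; Interactable side-by-side fridge whose freezer door, fridge door and door-in-door panel each open and close on interaction.
; OnInteraction checks the hit component's LeftDoor, RightDoor or InDoor tag to pick which door to move.
; Each door has its own FlipFlop that plays or reverses a timeline, lerping the mesh's relative yaw to swing it open in its hinge direction while keeping roll and pitch.
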(event Collision|EventActorBeginOverlap
  (params (OtherActor :type Actor%20Object%20Reference)))

(event EventOnInteraction
  (params (PrimRef :type Primitive%20Component%20Object%20Reference))
  (bind _sm_ka_f1000_fridgesbs_v1_frezzerdoor (Variables|Default|GetSM_KA-F1000_FridgeSBS_V1_FrezzerDoor))
  (bind _sm_ka_f1000_fridgesbs_v1_door (Variables|Default|GetSM_KA-F1000_FridgeSBS_V1_Door))
  (bind _sm_ka_f1000_fridgesbs_v1_doorindoor (Variables|Default|GetSM_KA-F1000_FridgeSBS_V1_DoorInDoor))
  (bind _returnvalue (Transformation|GetRelativeTransform _sm_ka_f1000_fridgesbs_v1_frezzerdoor))
  (bind _returnvalue_2 (Transformation|GetRelativeTransform _sm_ka_f1000_fridgesbs_v1_door))
  (bind _returnvalue_3 (Transformation|GetRelativeTransform _sm_ka_f1000_fridgesbs_v1_doorindoor))
  (if (Components|ComponentHasTag PrimRef "LeftDoor")
    (Utilities|FlowControl|FlipFlop
      (:A
        (bind _newtrack_0 (Timeline|Timeline Play)
          (:Update
            (Transformation|SetRelativeRotation _sm_ka_f1000_fridgesbs_v1_frezzerdoor (Math|Rotator|MakeRotator (.roll (.rotation _returnvalue)) (.pitch (.rotation _returnvalue)) (Math|Float|Lerp 0.0 1.4e+02 _newtrack_0)) false false))))
      (:B
        (Timeline|Timeline Reverse)))
    (elif (Components|ComponentHasTag PrimRef "RightDoor")
      (Utilities|FlowControl|FlipFlop
        (:A
          (bind _newtrack_0_2 (Timeline|Timeline_0 Play)
            (:Update
              (Transformation|SetRelativeRotation _sm_ka_f1000_fridgesbs_v1_door (Math|Rotator|MakeRotator (.roll (.rotation _returnvalue_2)) (.pitch (.rotation _returnvalue_2)) (Math|Float|Lerp 0.0 -1.4e+02 _newtrack_0_2)) false false))))
        (:B
          (Timeline|Timeline_0 Reverse)))
      (elif (Components|ComponentHasTag PrimRef "InDoor")
        (Utilities|FlowControl|FlipFlop
          (:A
            (bind _newtrack_0_3 (Timeline|Timeline_1 Play)
              (:Update
                (Transformation|SetRelativeRotation _sm_ka_f1000_fridgesbs_v1_doorindoor (Math|Rotator|MakeRotator (.roll (.rotation _returnvalue_3)) (.pitch (.rotation _returnvalue_3)) (Math|Float|Lerp 0.0 -1.4e+02 _newtrack_0_3)) false false))))
          (:B
            (Timeline|Timeline_1 Reverse)))))))

(fn ConstructionScript)